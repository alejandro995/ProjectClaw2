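; BP_Wall is a Paper2D wall actor that scrolls upward and removes itself.
; On BeginPlay it starts a Timeline, used as an update driver, that sets the actor location from the PaperFlipbook's world position plus WallVelocity in Z, keeping rotation.
; The step is per update without delta-time scaling, and the actor is destroyed once the flipbook rises above a fixed height.
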(event `self.ReceiveBeginPlay`
  (bind (_returnvalue_x _returnvalue_y _returnvalue_z) (`KismetMathLibrary.BreakVector` (`SceneComponent.K2_GetComponentLocation` (`self.PaperFlipbook`))))
  (`Timeline|Timeline` :`NewTime` 20.0
    (:`Update`
      (`self.K2_SetActorLocationAndRotation` (`KismetMathLibrary.MakeVector` _returnvalue_x _returnvalue_y (+ _returnvalue_z (`self.WallVelocity`))) (`self.K2_GetActorRotation` self))
      (if (> _returnvalue_z 800.0)
        (`self.K2_DestroyActor`)))))

(fn `UserConstructionScript`)