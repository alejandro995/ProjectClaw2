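; BP_Location is a platform spawner that places BP_Platform actors at random in one of three lanes.
; A Timeline starts on BeginPlay, with one track setting a Delay that throttles its updates into spawn intervals and another setting platform velocity.
; Each spawn cycle also adds the truncated velocity value to the player's Credits in BP_OsoPlayerState, then moves the Sphere to the chosen lane as the spawn point.
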(event `self.ReceiveBeginPlay`
  (bind (_returnvalue_location _returnvalue_rotation) (`KismetMathLibrary.BreakTransform` (`SceneComponent.K2_GetComponentToWorld` (`self.Sphere`))))
  (bind (_direction _newtrack_2 _newtrack_3) (`Timeline|Timeline`)
    (:`Update`
      (`KismetSystemLibrary.Delay` _newtrack_2)
      (bind _asbp_oso_player_state (cast `/Game/Character/State/BP_OsoPlayerState` (`Controller.PlayerState` (`GameplayStatics.GetPlayerController` 0))))
      (set `/Game/Character/State/BP_OsoPlayerState.Credits` (+ (`/Game/Character/State/BP_OsoPlayerState.Credits` _asbp_oso_player_state) (`KismetMathLibrary.FTrunc` _newtrack_3)) _asbp_oso_player_state)
      (switch `int` (`KismetMathLibrary.RandomIntegerInRange` 0 2)
        (:`0`
          (`SceneComponent.K2_SetWorldLocation` (`self.Sphere`) (-70.0 0.0 100.0) false false))
        (:`1`
          (`SceneComponent.K2_SetWorldLocation` (`self.Sphere`) (0.0 0.0 100.0) false false))
        (:`2`
          (`SceneComponent.K2_SetWorldLocation` (`self.Sphere`) (70.0 0.0 100.0) false false)))
      (bind _returnvalue (`|SpawnActorFromClass` "/Game/BluePrints/Platforms/BP_Platform.BP_Platform_C" (`KismetMathLibrary.MakeTransform` _returnvalue_location _returnvalue_rotation (0.45 1.0 0.45)) "Undefined" "OverrideRootScale" null null))
      (set `/Game/BluePrints/Platforms/BP_Platform.velocity` _newtrack_3 _returnvalue))))

(fn `GetRandomPlatform`
  (params (CurrentPlatform :type Integer))
  (returns (NewPlatform :type Integer))
  (return 0))

(fn `UserConstructionScript`)