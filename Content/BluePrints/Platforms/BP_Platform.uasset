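; BP_Platform is a sprite-based platform that moves along the Z axis and removes itself on reaching a trigger volume.
; A Timeline started on BeginPlay acts as a tick, adding Velocity to the sprite's world Z on each update, so speed depends on frame rate.
; Overlapping a TriggerVolume destroys the actor, while the Character overlap branch is an empty stub.
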(event `self.ReceiveBeginPlay`
  (bind (_returnvalue_x _returnvalue_y _returnvalue_z) (`KismetMathLibrary.BreakVector` (`SceneComponent.K2_GetComponentLocation` (`self.PlatformSprite`))))
  (`Timeline|Timeline` :`NewTime` 20.0
    (:`Update`
      (`self.K2_SetActorLocationAndRotation` (`KismetMathLibrary.MakeVector` _returnvalue_x _returnvalue_y (+ _returnvalue_z (`self.velocity`))) (`self.K2_GetActorRotation` self)))))

(event `self.PlatformSprite.OnComponentBeginOverlap`
  (params (OverlappedComponent :type "PrimitiveComponent Object Reference") (OtherActor :type "Actor Object Reference") (OtherComp :type "PrimitiveComponent Object Reference") (OtherBodyIndex :type Integer) (bFromSweep :type Boolean) (SweepResult :type "HitResult Structure (by ref)"))
  (bind _ascharacter (cast `Character` OtherActor)
    (:`then`
      (`/Engine/EditorBlueprintResources/StandardMacros.IsValid` _ascharacter))
    (:`CastFailed`
      (bind _astrigger_volume (cast `TriggerVolume` OtherActor))
      (`/Engine/EditorBlueprintResources/StandardMacros.IsValid` _astrigger_volume
        (:`Is Valid`
          (`self.K2_DestroyActor`))))))

(fn `UserConstructionScript`)