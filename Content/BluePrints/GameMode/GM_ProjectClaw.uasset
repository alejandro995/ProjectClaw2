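; Game mode for Project Claw that starts the music, sets up the player camera and handles respawning.
; At play start it turns the sprite character to a fixed yaw and blends the view to the level's BP_CharacterCamera actor.
; RespawnPlayer spawns a new pawn of the given player's class at SpawnTransform, possesses it, reapplies the camera setup and flags Respawn on BP_OsoPlayerState.
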(event `self.ReceiveBeginPlay`
  (`self.AttachToCamera`)
  (`GameplayStatics.PlaySound2D` "/Game/Assets/Sound/Power_-_DNB.Power_-_DNB" 1.0 1.0 0.0 null null))

(event `Respawn Player`
  (params (player :type "Character Object Reference"))
  (bind _returnvalue (`GameplayStatics.GetPlayerController` 0))
  (bind _returnvalue_2 (`|SpawnActorFromClass` (`GameplayStatics.GetObjectClass` player) (`self.Spawn Transform`) "Undefined" "OverrideRootScale" null null))
  (`Controller.Possess` _returnvalue _returnvalue_2)
  (`self.AttachToCamera`)
  (bind _asbp_oso_player_state (cast `/Game/Character/State/BP_OsoPlayerState` (`Controller.PlayerState` _returnvalue)))
  (set `/Game/Character/State/BP_OsoPlayerState.Respawn` true _asbp_oso_player_state))

(event `AttachToCamera`
  (bind _asbp_sprite_character (cast `/Game/Character/BP_SpriteCharacter` (`GameplayStatics.GetPlayerCharacter` 0)))
  (if (`KismetSystemLibrary.IsValid` _asbp_sprite_character)
    (`self.K2_SetActorRotation` _asbp_sprite_character (struct :`Yaw` -90.0) false)
    (bind _asplayer_controller (cast `PlayerController` (`Pawn.GetController` _asbp_sprite_character)))
    (if (`KismetSystemLibrary.IsValid` _asplayer_controller)
      (bind _returnvalue (`GameplayStatics.GetActorOfClass` "/Game/Character/Camera/BP_CharacterCamera.BP_CharacterCamera_C"))
      (`PlayerController.SetViewTargetWithBlend` _asplayer_controller _returnvalue 0.5 "VTBlend_Linear" 0.0 false))))

(fn `UserConstructionScript`)